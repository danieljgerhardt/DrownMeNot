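; Blast projectile actor for the Gameplay Ability System that reports when it overlaps something other than its owner.
; Launch makes both spheres and the owner's capsule ignore each other while moving, then feeds player 0's camera forward vector into the projectile movement's local-space velocity at a fixed speed.
; A Sphere1 overlap calls the ProjectileConnected dispatcher, with no damage or effect applied in this graph.
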(event OnComponentBeginOverlap(Sphere1)
  (params (OverlappedComponent :type Primitive%20Component%20Object%20Reference) (OtherActor :type Actor%20Object%20Reference) (OtherComp :type Primitive%20Component%20Object%20Reference) (OtherBodyIndex :type Integer) (bFromSweep :type Boolean) (SweepResult :type Hit%20Result%20Structure%20%28by%20ref%29))
  (if (!= OtherActor (Components|GetOwner))
    (Default|CallProjectileConnectedDispatcher)))

(event Custom|Launch
  (CallFunction|SetupIgnore)
  (Utilities|IsValid (Components|GetOwner)
    (:Is%20Valid
      (Game|Components|ProjectileMovement|SetVelocityinLocalSpace (Variables|Default|GetProjectileMovement) (* (Math|Vector|GetForwardVector (Variables|/Script/Engine.PlayerCameraManager|GetTransformComponent (Game|GetPlayerCameraManager 0))) 2e+03)))))

(event EventBeginPlay)

(event Collision|EventActorBeginOverlap
  (params (OtherActor :type Actor%20Object%20Reference)))

(event EventTick
  (params (DeltaSeconds :type Float%20%28single-precision%29)))

(fn ConstructionScript)

(fn SetupIgnore
  (bind _returnvalue (Components|GetOwner))
  (Collision|IgnoreActorwhenMoving (Variables|Default|GetSphere1) _returnvalue true)
  (Collision|IgnoreActorwhenMoving (Actor|GetComponentbyClass _returnvalue "/Script/Engine.CapsuleComponent") self true)
  (Collision|IgnoreActorwhenMoving (Variables|Default|GetSphere) _returnvalue true))