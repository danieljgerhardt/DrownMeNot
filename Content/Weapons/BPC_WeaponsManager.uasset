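; Weapons manager component for a CharacterBase owner that equips and unequips a single weapon at a time.
; EquipWeapon spawns the requested class and attaches it to the mesh socket named in its WeaponConfig, replacing the current weapon or toggling it off if the same class is requested.
; Each weapon's config drives the anim class and movement settings, while unequipping destroys the actor and restores ABP_Unarmed and the unequipped movement properties.
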(event Custom|Equip%20Weapon
  (params (Weapon%20Class :type BP%20Weapon%20Base%20Class%20Reference))
  (bind _character (Variables|Default|GetCharacter))
  (bind _charactermovement (Variables|/Script/Engine.Character|GetCharacterMovement _character))
  (Variables|Default|GetCharacter
    (:then
      (bind _equipped_weapon (Variables|Default|GetEquipped%20Weapon)
        (:then
          (if (== (Utilities|GetClass _equipped_weapon) Weapon%20Class)
            (CallFunction|UnequipWeapon)
            (else
              (CallFunction|UnequipWeapon)
              (bind _returnvalue (Game|SpawnActorfromClass Weapon%20Class (Math|Transform|MakeTransform "0, 0, 0" "0, 0, 0" "1.000000,1.000000,1.000000") "Undefined" "MultiplyWithRoot" 0 0 :!label _label))
              (bind _output_get (Variables|Default|SetEquipped%20Weapon _returnvalue))
              (Transformation|AttachComponentToComponent _returnvalue (Variables|/Script/Engine.Character|GetMesh (Variables|Default|GetCharacter)) (.EquippedSocketName (Utilities|Struct|BreakS_WeaponConfig (Variables|/Game/Weapons/BP_Weapon_Base.BP_Weapon_Base_C|GetWeapon%20Config _output_get))) "SnapToTarget" "SnapToTarget" "SnapToTarget" true)
              (Components|SkeletalMesh|SetAnimInstanceClass (Variables|/Script/Engine.Character|GetMesh (Variables|Default|GetCharacter)) (.AnimClass (Utilities|Struct|BreakS_WeaponConfig (Variables|/Game/Weapons/BP_Weapon_Base.BP_Weapon_Base_C|GetWeapon%20Config (Variables|Default|GetEquipped%20Weapon)))))
              (Variables|/Script/Engine.CharacterMovementComponent|SetMaxWalkSpeed _charactermovement (.MaxWalkSpeed (Utilities|Struct|BreakS_WeaponMovementProperties (.MovementProperties (Utilities|Struct|BreakS_WeaponConfig (Variables|/Game/Weapons/BP_Weapon_Base.BP_Weapon_Base_C|GetWeapon%20Config (Variables|Default|GetEquipped%20Weapon)))))))
              (Variables|/Script/Engine.CharacterMovementComponent|SetbOrientRotationToMovement _charactermovement (.OrientRotationtoMovement (Utilities|Struct|BreakS_WeaponMovementProperties (.MovementProperties (Utilities|Struct|BreakS_WeaponConfig (Variables|/Game/Weapons/BP_Weapon_Base.BP_Weapon_Base_C|GetWeapon%20Config (Variables|Default|GetEquipped%20Weapon)))))))
              (Variables|/Script/Engine.CharacterMovementComponent|SetbUseControllerDesiredRotation _charactermovement (.UseControllerDesiredRotation (Utilities|Struct|BreakS_WeaponMovementProperties (.MovementProperties (Utilities|Struct|BreakS_WeaponConfig (Variables|/Game/Weapons/BP_Weapon_Base.BP_Weapon_Base_C|GetWeapon%20Config (Variables|Default|GetEquipped%20Weapon))))))))))
        (:else
          (goto _label))))
    (:else)))

(event Custom|Unequip%20Weapon
  (bind _character (Variables|Default|GetCharacter))
  (bind _unequipped_movement_properties (Variables|Default|GetUnequipped%20Movement%20Properties))
  (bind (_maxwalkspeed _orientrotationtomovement _usecontrollerdesiredrotation) (Utilities|Struct|BreakS_WeaponMovementProperties _unequipped_movement_properties))
  (bind _charactermovement (Variables|/Script/Engine.Character|GetCharacterMovement _character))
  (bind _equipped_weapon (Variables|Default|GetEquipped%20Weapon)
    (:then
      (Actor|DestroyActor _equipped_weapon)
      (Variables|Default|SetEquipped%20Weapon 0)
      (Components|SkeletalMesh|SetAnimInstanceClass (Variables|/Script/Engine.Character|GetMesh (Variables|Default|GetCharacter)) "/Game/Characters/Mannequins/Anims/Unarmed/ABP_Unarmed.ABP_Unarmed_C")
      (Variables|/Script/Engine.CharacterMovementComponent|SetMaxWalkSpeed _charactermovement _maxwalkspeed)
      (Variables|/Script/Engine.CharacterMovementComponent|SetbOrientRotationToMovement _charactermovement _orientrotationtomovement)
      (Variables|/Script/Engine.CharacterMovementComponent|SetbUseControllerDesiredRotation _charactermovement _usecontrollerdesiredrotation))
    (:else)))

(event EventBeginPlay
  (bind _ascharacter_base (Utilities|Casting|CastToCharacterBase (Components|GetOwner)))
  (Variables|Default|SetCharacter _ascharacter_base))