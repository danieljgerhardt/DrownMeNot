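; Sample character for sword animations that moves its static mesh, presumably the sword, between the Sheath and Weapon sockets on the skeletal mesh.
; Every Tick it polls the AnimInstance for active notify states and reattaches the mesh with keep-relative rules.
; Unsheath-start or Sheath states select the Sheath socket and take priority; Sheath-start or Unsheath states select the Weapon socket.
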(event EventBeginPlay)

(event Collision|EventActorBeginOverlap
  (params (OtherActor :type Actor%20Object%20Reference)))

(event EventTick
  (params (DeltaSeconds :type Float%20%28single-precision%29))
  (if (or (Class|AnimInstance|WasAnimNotifyStateActiveinAnyState (Components|SkeletalMesh|GetAnimInstance (Variables|Character|GetMesh)) "/Game/SwordAnims/Blueprint/BP_ANS_AnimStart_Unsheath.BP_ANS_AnimStart_Unsheath_C") (Class|AnimInstance|WasAnimNotifyStateActiveinAnyState (Components|SkeletalMesh|GetAnimInstance (Variables|Character|GetMesh)) "/Game/SwordAnims/Blueprint/BP_ANS_Sheath.BP_ANS_Sheath_C"))
    (Transformation|AttachComponentToComponent (Variables|Default|GetStaticMesh) (Variables|Character|GetMesh) "Sheath" "KeepRelative" "KeepRelative" "KeepRelative" true)
    (elif (or (Class|AnimInstance|WasAnimNotifyStateActiveinAnyState (Components|SkeletalMesh|GetAnimInstance (Variables|Character|GetMesh)) "/Game/SwordAnims/Blueprint/BP_ANS_AnimStart_Sheath.BP_ANS_AnimStart_Sheath_C") (Class|AnimInstance|WasAnimNotifyStateActiveinAnyState (Components|SkeletalMesh|GetAnimInstance (Variables|Character|GetMesh)) "/Game/SwordAnims/Blueprint/BP_ANS_Unsheath.BP_ANS_Unsheath_C"))
      (Transformation|AttachComponentToComponent (Variables|Default|GetStaticMesh) (Variables|Character|GetMesh) "Weapon" "KeepRelative" "KeepRelative" "KeepRelative" true))))

(fn ConstructionScript)